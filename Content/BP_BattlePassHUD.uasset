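; Battle Pass HUD that puts the Battle Pass reward screen on the player's viewport when play begins.
; BeginPlay creates W_BattlePass, shows the mouse cursor and fills the widget from RewardData.
; It then calls CallOnNewLevelGained on BP_BattlePassPlayerController with level 1 to refresh the slots' look.
; SetupInput can add the default Enhanced Input mapping context but is not called here, and the CreateWidget function is an empty stub.
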(event EventBeginPlay
  (bind _returnvalue (Game|GetPlayerController 0))
  (Utilities|FlowControl|Sequence
    (:then_0
      ;[0 0 0 0.5] Create and show Battle Pass Widget
      (bind _returnvalue_2 (UserInterface|CreateWidget "/Game/UI/BattlePass/W_BattlePass.W_BattlePass_C" _returnvalue))
      (bind _output_get (Variables|Default|SetBattlePassWidget _returnvalue_2))
      (UserInterface|Viewport|AddtoViewport _output_get 0)
      (Variables|/Script/Engine.PlayerController|SetbShowMouseCursor _returnvalue true)
      (Default|InitRewards (Variables|Default|GetBattlePassWidget) (Variables|Default|GetRewardData)))
    (:then_1
      ;[0 0 0 0.5] Call to refresh slots look
      (bind _asbp_battle_pass_player_controller (Utilities|Casting|CastToBP_BattlePassPlayerController (Game|GetPlayerController 0)))
      (Default|CallOnNewLevelGained _asbp_battle_pass_player_controller 1))))

(fn ConstructionScript)

(fn CreateWidget
  (params (Class :type User%20Widget%20Class%20Reference) (bShowMouseCursor :type Boolean)))

(fn SetupInput
  (bind _returnvalue (Game|GetPlayerController 0))
  (bind _returnvalue_2 (PlayerController|LocalPlayerSubsystems|GetEnhancedInputLocalPlayerSubsystem _returnvalue))
  (Utilities|IsValid _returnvalue_2
    (:Is%20Valid
      (Input|AddMappingContext _returnvalue_2 "/Game/Input/IMC_Default.IMC_Default" 0 "(bIgnoreAllPressedKeysUntilRelease=True,bForceImmediately=False,bNotifyUserSettings=False)"))))